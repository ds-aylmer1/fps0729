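; Monster enemy AI for an FPS that wanders randomly until it senses or is shot by the player, then chases them.
; A looping AIMoveTo drives movement; reaching the player pauses it for a timed attack that briefly enables the attack area's overlap events to deal damage.
; Bullet overlaps on the capsule subtract health; death ragdolls the mesh, increments the game mode's kill count and destroys the actor after a delay.
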(event `self.感測元件.OnSeePawn`
  (params (Pawn :type "Pawn Object Reference"))
  (bind `_攻擊區域` (`self.攻擊區域`))
  (bind _charactermovement (`self.CharacterMovement`))
  ;[1 0.8173 0.1003] 看到玩家後保存玩家資訊
  (bind _asbp_fps_player_content (cast `/Game/FPS_BP_Pereson/BP_FPS_player` Pawn))
  (set `self.As BP FPS Player` _asbp_fps_player_content)
  (set `self.是否看到玩家` true :!label _label)
  (set `self.停留時間最大值` 0.0) ; 看到玩家後馬上往玩家前進
  (`/Engine/EditorBlueprintResources/StandardMacros.DoOnce` false ; 執行一次
    (:`Completed`
      ;[1 0.6718 0.4989] 判斷有沒有看到玩家:
      ; 有的畫朝上面藍圖走沒有朝下面走
      (if (`self.是否看到玩家`) :!label _label_2
        ;[0.3229 0.6557 1] 看到玩家後:追蹤玩家
        (`|AIMoveTo` self (0.0 0.0 0.0) (`self.As BP FPS Player`) (`self.停止半徑`)
          (:`OnSuccess`
            ;[1 0.4725 0.3524] 攻擊狀態
            (set `self.怪物攻擊中` true)
            (set `CharacterMovementComponent.MaxWalkSpeed` 0.0 _charactermovement)
            (`KismetSystemLibrary.Delay` 3.0) ; 手舉起來時間
            (set `PrimitiveComponent.bGenerateOverlapEvents` true `_攻擊區域`) ; 開啟碰撞
            (`KismetSystemLibrary.Delay` 0.5) ; 碰撞停留時間
            (set `PrimitiveComponent.bGenerateOverlapEvents` false `_攻擊區域`) ; 關閉碰撞
            (`KismetSystemLibrary.Delay` 1.0) ; 動畫完畢後
            (set `CharacterMovementComponent.MaxWalkSpeed` 500.0 _charactermovement)
            (set `self.怪物攻擊中` false)
            (goto _label_2))
          (:`OnFail`
            (set `self.是否看到玩家` false)
            (set `self.停留時間最大值` 3.0) ; 恢復停留最大值為 3
            (goto _label_2)))
        (else
          ;[0.4223 0.7531 1] 沒看到玩家:隨機走動
          (`|AIMoveTo` self (`NavigationSystemV1.K2_GetRandomReachablePointInRadius` (`SceneComponent.K2_GetComponentLocation` (`self.CapsuleComponent`)) (`self.隨機走動的半徑`) null null) null (`self.停止半徑`) ; AI移動節點:移動到指定的座標
            (:`then`
              ;[0.4223 0.7531 1] 隨機停留
              (`KismetSystemLibrary.Delay` (* (`KismetMathLibrary.RandomFloat`) (`self.停留時間最大值`)))
              (goto _label_2))))))))

(event `self.ReceiveBeginPlay`
  (`|ExecutionSequence`
    (:`then_0`
      (goto _label_2))
    (:`then_1`
      ;[1 1 1] 取得遊戲模式
      (bind _asbp_fps_player_mod (cast `/Game/FPS_BP_Pereson/BP_FPS_player_MOD` (`GameplayStatics.GetGameMode`)))
      (set `self.As BP FPS Player Control` _asbp_fps_player_mod))
    (:`then_2`
      ;[0.302 1 0.3919] 忽略碰撞
      (`PrimitiveComponent.IgnoreComponentWhenMoving` (`self.CapsuleComponent`) (`self.攻擊區域`) false))
    (:`then_3`
      ;[1 1 1] 取得玩家藍圖
      (bind _asbp_fps_player (cast `/Game/FPS_BP_Pereson/BP_FPS_player` (`GameplayStatics.GetPlayerCharacter` 0)))
      (set `self.As BP FPS Player` _asbp_fps_player))))

(event `self.CapsuleComponent.OnComponentBeginOverlap`
  (params (OverlappedComponent :type "PrimitiveComponent Object Reference") (OtherActor :type "Actor Object Reference") (OtherComp :type "PrimitiveComponent Object Reference") (OtherBodyIndex :type Integer) (bFromSweep :type Boolean) (SweepResult :type "HitResult Structure (by ref)"))
  (bind _as_bp_fps_player_control (`self.As BP FPS Player Control`))
  ;[1 0.1946 0.2643] 受傷與死亡
  (bind `_asbp_子彈bullet` (cast `/Game/FPS_BP_Pereson/BP_子彈Bullet` OtherActor))
  (bind `_目前武器傷害` (`/Game/FPS_BP_Pereson/BP_子彈Bullet.目前武器傷害` `_asbp_子彈bullet`))
  ;[1 1 1] 測試受傷顯示
  (`KismetSystemLibrary.PrintString` (`KismetStringLibrary.Conv_DoubleToString` `_目前武器傷害`))
  (bind `_是否死亡` (`self.受傷` `_目前武器傷害`))
  (if `_是否死亡`
    (set `/Game/FPS_BP_Pereson/BP_FPS_player_MOD.殺怪物數量 monters Number` (+ (`/Game/FPS_BP_Pereson/BP_FPS_player_MOD.殺怪物數量 monters Number` _as_bp_fps_player_control) 1) _as_bp_fps_player_control)
    (`KismetSystemLibrary.Delay` 5.0)
    (`self.K2_DestroyActor`)
    (else
      (goto _label))))

(event `self.攻擊區域.OnComponentBeginOverlap`
  (params (OverlappedComponent :type "PrimitiveComponent Object Reference") (OtherActor :type "Actor Object Reference") (OtherComp :type "PrimitiveComponent Object Reference") (OtherBodyIndex :type Integer) (bFromSweep :type Boolean) (SweepResult :type "HitResult Structure (by ref)"))
  ;[1 0.1435 0.8422] 攻擊區域判定與傳送傷害
  (bind _asbp_fps_player_content (cast `/Game/FPS_BP_Pereson/BP_FPS_player` OtherActor))
  (`/Game/FPS_BP_Pereson/BP_FPS_player.受傷` _asbp_fps_player_content (`self.怪物攻擊力量`)))

(fn `UserConstructionScript`)

(fn `受傷`
  (params (`接收到傷害值` :type "Float (double-precision)"))
  (returns (`是否死亡` :type Boolean))
  ;[1 1 1] 受傷
  (bind _output_get (set `self.血量` (- (`self.血量`) `接收到傷害值`)))
  (if (<= _output_get 0.0)
    ;[1 0.07764 0] 死亡
    (`PrimitiveComponent.SetSimulatePhysics` (`self.Mesh`) true) ; 模擬布偶物理效果
    (`PrimitiveComponent.SetCollisionEnabled` (`self.CapsuleComponent`) "NoCollision") ; 設定碰撞啟動:關閉膠囊碰撞避免產生太大碰撞
    (return true)
    (else
      (return false))))