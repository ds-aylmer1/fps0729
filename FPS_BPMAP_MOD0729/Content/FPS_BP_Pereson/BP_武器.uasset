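; Player weapon actor (SKAR4 model) for an FPS, handling automatic fire, magazine reloading and ammo pickup.
; The fire input, gated on press by the player's reload and sprint states, starts a Delay loop until release or empty magazine.
; Each shot spawns a bullet at the muzzle socket, passes it damage and plays a muzzle flash.
; Custom events refill the magazine from reserve ammo and add one magazine to the capped reserve.
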(event `self.ReceiveBeginPlay`
  ;[1 1 1] 取得玩家資訊
  (bind _asbp_fps_player_content (cast `/Game/FPS_BP_Pereson/BP_FPS_player` (`GameplayStatics.GetPlayerCharacter` 0)))
  (set `self.玩家控制` _asbp_fps_player_content))

(event `InputAction|開槍`
  (params (Key :type "Key Structure"))
  (bind `_武器模型sk_ar4` (`self.武器模型SK_AR4`))
  (bind `_玩家控制` (`self.玩家控制`))
  (bind (_returnvalue_roll _returnvalue_pitch _returnvalue_yaw) (`KismetMathLibrary.BreakRotator` (`SceneComponent.GetSocketRotation` `_武器模型sk_ar4` "None")))
  ;[1 1 1] 開槍功能
  (:`Pressed`
    (if (and (not (`/Game/FPS_BP_Pereson/BP_FPS_player.換彈夾` `_玩家控制`)) (not (`/Game/FPS_BP_Pereson/BP_FPS_player.衝刺` `_玩家控制`)))
      (set `self.開槍中` true)
      (if (and (> (`self.目前子彈數量Current number of  bullets`) 0) (`self.開槍中`)) :!label _label
        (bind _returnvalue (`|SpawnActorFromClass` "/Game/FPS_BP_Pereson/BP_子彈Bullet.BP_子彈Bullet_C" (`SceneComponent.GetSocketTransform` (`self.武器模型SK_AR4`) "Bullet子彈插槽" "RTS_World") "Undefined" "OverrideRootScale" null null)) ; 生成子彈藍圖
        (set `/Game/FPS_BP_Pereson/BP_子彈Bullet.目前武器傷害` (`self.武器傷害`) _returnvalue) ; 將武器傷害轉給子彈
        (`GameplayStatics.SpawnEmitterAtLocation` "/Game/InfinityBladeEffects/Effects/FX_Monsters/FX_Monster_Gruntling/Master/P_BackPack_MuzzleFlash.P_BackPack_MuzzleFlash" (`SceneComponent.GetSocketLocation` `_武器模型sk_ar4` "Bullet子彈插槽") (`KismetMathLibrary.MakeRotator` (+ _returnvalue_roll 90.0) (+ _returnvalue_pitch 5.0) (+ _returnvalue_yaw 180.0)) (0.01 0.01 0.01)) ; 生成粒子在指定的座標上
        (set `self.目前子彈數量Current number of  bullets` (- (`self.目前子彈數量Current number of  bullets`) 1)) ; 開槍後子彈數量-1
        (`KismetSystemLibrary.Delay` (`self.開槍間隔`))
        (goto _label))))
  (:`Released`
    (set `self.開槍中` false)))

(event `換彈夾`
  ;[0.1312 1 0.4542] 計算要補充幾顆子彈
  (set `self.要補充的子彈數量` (- (`self.彈匣尺寸容量`) (`self.目前子彈數量Current number of  bullets`))) ; 計算要補充的數量 : \n範例 目前 10 但夾30 所以要補充20
  ;[0.4691 1 0.1779] 判斷總數是否大於等於要補充的數量
  (if (not (>= (`self.子彈總數 Total number of bullets`) (`self.要補充的子彈數量`)))
    ;[0.1142 1 0.3919] 總數<要補充的數量:把剩餘總數補充
    (set `self.要補充的子彈數量` (`self.子彈總數 Total number of bullets`)))
  ;[0.1142 1 0.2793] 目前子彈以及總數更新
  (set `self.目前子彈數量Current number of  bullets` (+ (`self.目前子彈數量Current number of  bullets`) (`self.要補充的子彈數量`))) ; 補充子彈數量,例:目前10要補充為 20 補充 後    目前為30
  (set `self.子彈總數 Total number of bullets` (- (`self.子彈總數 Total number of bullets`) (`self.要補充的子彈數量`))) ; 扣除子彈總數,\n例: 總數20要補充為20 補充後 總數為0
)

(event `補充子彈`
  ;[0.1514 1 0.3143] 補充子彈系統
  (bind _output_get (set `self.子彈總數 Total number of bullets` (+ (`self.子彈總數 Total number of bullets`) (`self.彈匣尺寸容量`)))) ; 子彈總數+彈匣尺寸
  (set `self.子彈總數 Total number of bullets` (`KismetMathLibrary.Clamp` _output_get 0 (`self.子彈上限`))))

(fn `UserConstructionScript`)